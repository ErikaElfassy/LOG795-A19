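; MyRosettaCharacter is a character Blueprint that links dialogue callbacks to quest progress and response checking.
; OnDialogueEvent switches on the event name to begin IntroQuest and update its Finn steps, or to call ResponseResult then CompareResponse for Finn's answer.
; GetBoolValue reports IntroQuest completion from QuestStatus back to dialogue.
; The event graph and construction script hold no logic.
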(event EventBeginPlay)

(event Collision|EventActorBeginOverlap
  (params (OtherActor :type Actor%20Object%20Reference)))

(event EventTick
  (params (DeltaSeconds :type Float%20%28single-precision%29)))

(fn ConstructionScript)

(fn OnDialogueEvent
  (params (EventName :type Name%20%28by%20ref%29 :default "None"))
  (|SwitchDialogueCallbackEvent EventName
    (:Default
      _)
    (:AnswerFinn
      (Class|RosettaCharacter|ResponseResult)
      (Class|RosettaCharacter|CompareResponse))
    (:ConcludeIntroQuest
      (Class|QuestStatus|UpdateQuests (Variables|Default|GetQuestStatus) "/Game/Quests/Intro/InputAtoms/IQ_AnswerFinn.IQ_AnswerFinn"))
    (:TalkToFinn
      (Class|QuestStatus|BeginQuest (Variables|Default|GetQuestStatus) "/Game/Quests/IntroQuest.IntroQuest")
      (Class|QuestStatus|UpdateQuests (Variables|Default|GetQuestStatus) "/Game/Quests/Intro/InputAtoms/IQ_TalkToFinn.IQ_TalkToFinn")))
  (return false))

(fn GetBoolValue
  (params (ValueName :type Name%20%28by%20ref%29 :default "None"))
  (|SwitchDialogueCallbackBoolValue ValueName
    (:Default
      _)
    (:QuestIsCompleted
      (bind _returnvalue (Class|QuestStatus|QuestIsCompleted (Variables|Default|GetQuestStatus) "/Game/Quests/IntroQuest.IntroQuest"))))
  (return _returnvalue))